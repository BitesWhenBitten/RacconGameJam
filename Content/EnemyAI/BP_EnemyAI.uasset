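; Enemy AI that patrols between two points, chases the raccoon player and flags Caught on the GameMode on contact.
; PawnSensing sight or timer-polled hearing triggers chases, with nested Running, Walking and Crouching overlap volumes checked against player movement state.
; Looping timers drive patrol, hearing and repeated chase moves.
; Losing the player starts searches at random nearby navigable points before patrol resumes.
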(event `self.PawnSensing.OnSeePawn`
  (params (Pawn :type "Pawn Object Reference"))
  ;[1 1 1] Ai Sight
  (cast `/Game/ThirdPerson/Blueprints/BP_RaccoonCharacter` Pawn)
  (`self.Aisee`))

(event `Aisee`
  ;[1 1 1] Sight Chase Start
  (set `self.Searching` false)
  (`|ExecutionSequence`
    (:`then_0`
      (set `self.chasing` true)
      (`|AIMoveTo` self (`self.K2_GetActorLocation` (`GameplayStatics.GetPlayerCharacter` 0)) null))
    (:`then_1`
      (`KismetSystemLibrary.RetriggerableDelay` 2.0)
      (if (`PrimitiveComponent.IsOverlappingActor` (`self.r`) (`GameplayStatics.GetPlayerCharacter` 0))
        (`self.Aisee`)
        (else
          (set `self.chasing` false)
          (`self.Lost Search`))))))

(event `Lost Search`
  ;[1 1 1] Search
  (if (not (`self.chasing`))
    (set `self.Searching` true)
    (`|ExecutionSequence`
      (:`then_0`
        (`KismetSystemLibrary.Delay` 1.0)
        (bind _randomlocation (`NavigationSystemV1.K2_GetRandomLocationInNavigableRadius` (`self.K2_GetActorLocation`) 500.0 null null))
        (`|AIMoveTo` self _randomlocation null 20.0
          (:`OnSuccess`
            (`KismetSystemLibrary.PrintString` "searching AA"))
          (:`OnFail`
            (`KismetSystemLibrary.PrintString` "fail searching" :!label _label)
            (set `self.Searching` false :!label _label_2)
            (`KismetSystemLibrary.PrintString` "searching BB"))))
      (:`then_1`
        (`KismetSystemLibrary.Delay` 5.0)
        (bind _randomlocation_2 (`NavigationSystemV1.K2_GetRandomLocationInNavigableRadius` (`self.K2_GetActorLocation`) 500.0 null null))
        (`|AIMoveTo` self _randomlocation_2 null 20.0
          (:`OnSuccess`
            (goto _label_2))
          (:`OnFail`
            (goto _label)))))))

(event `self.catching.OnComponentBeginOverlap`
  (params (OverlappedComponent :type "PrimitiveComponent Object Reference") (OtherActor :type "Actor Object Reference") (OtherComp :type "PrimitiveComponent Object Reference") (OtherBodyIndex :type Integer) (bFromSweep :type Boolean) (SweepResult :type "HitResult Structure (by ref)"))
  ;[1 1 1] Catch code
  (if (== OtherActor (`GameplayStatics.GetPlayerCharacter` 0))
    (bind _asbp_raccoon_game_jam_game_mode (cast `/Game/GameModes/BP_RaccoonGameJamGameMode` (`GameplayStatics.GetGameMode`)))
    (set `/Game/GameModes/BP_RaccoonGameJamGameMode.Caught` true _asbp_raccoon_game_jam_game_mode)
    (`KismetSystemLibrary.PrintString` "CAUGHT")
    (else
      (`KismetSystemLibrary.PrintString` "Failed"))))

(event `self.running.OnComponentEndOverlap`
  (params (OverlappedComponent :type "PrimitiveComponent Object Reference") (OtherActor :type "Actor Object Reference") (OtherComp :type "PrimitiveComponent Object Reference") (OtherBodyIndex :type Integer))
  ;[1 1 1] Escape Check
  (if (`self.chasing`)
    (set `self.chasing` false)
    (`KismetSystemLibrary.PrintString` "OUTSIDE RANGE")
    (`self.Lost Search`)))

(event `self.ReceiveBeginPlay`
  (`KismetSystemLibrary.K2_SetTimerDelegate` (delegate `Patrol`) 5.0 true)
  (`KismetSystemLibrary.K2_SetTimerDelegate` (delegate `Hearing`) 0.1 true)
  (`KismetSystemLibrary.K2_SetTimerDelegate` (delegate `Chasetime`) 0.1 true))

(event `Patrol`
  ;[1 1 1] Patrol
  (if (`self.chasing`)
    _
    (elif (not (`self.Searching`))
      (`KismetSystemLibrary.PrintString` "Patrolling")
      (`/Engine/EditorBlueprintResources/StandardMacros.FlipFlop`
        (:`A`
          (`|AIMoveTo` self (`self.K2_GetActorLocation` (`self.Patrol Point 1`)) null))
        (:`B`
          (`|AIMoveTo` self (`self.K2_GetActorLocation` (`self.Patrol Point 2`)) null))))))

(event `Hearing`
  ;[1 1 1] AI Hearing
  (if (`PrimitiveComponent.IsOverlappingActor` (`self.running`) (`GameplayStatics.GetPlayerCharacter` 0))
    (bind _asbp_raccoon_character (cast `/Game/ThirdPerson/Blueprints/BP_RaccoonCharacter` (`GameplayStatics.GetPlayerCharacter` 0)))
    (if (`NavMovementComponent.IsMovingOnGround` (`Character.CharacterMovement` _asbp_raccoon_character))
      (if (`/Game/ThirdPerson/Blueprints/BP_RaccoonCharacter.sprinting` _asbp_raccoon_character)
        (set `self.chasing` true)
        (else
          (if (`PrimitiveComponent.IsOverlappingActor` (`self.walking`) (`GameplayStatics.GetPlayerCharacter` 0)) :!label _label_3
            (bind _asbp_raccoon_character_2 (cast `/Game/ThirdPerson/Blueprints/BP_RaccoonCharacter` (`GameplayStatics.GetPlayerCharacter` 0)))
            (if true
              (if (`/Game/ThirdPerson/Blueprints/BP_RaccoonCharacter.crouching` _asbp_raccoon_character_2)
                (if (`PrimitiveComponent.IsOverlappingActor` (`self.crouching`) (`GameplayStatics.GetPlayerCharacter` 0)) :!label _label_4
                  (bind _asbp_raccoon_character_3 (cast `/Game/ThirdPerson/Blueprints/BP_RaccoonCharacter` (`GameplayStatics.GetPlayerCharacter` 0)))
                  (if (`NavMovementComponent.IsMovingOnGround` (`Character.CharacterMovement` _asbp_raccoon_character_3))
                    (if (`/Game/ThirdPerson/Blueprints/BP_RaccoonCharacter.crouching` _asbp_raccoon_character_3)
                      (set `self.chasing` true))))
                (else
                  (set `self.chasing` true)))
              (else
                (goto _label_4)))
            (else
              (goto _label_4)))))
      (else
        (goto _label_3)))
    (else
      (goto _label_3))))

(event `Chasetime`
  (bind _returnvalue (`GameplayStatics.GetPlayerCharacter` 0))
  ;[1 1 1] Chasing
  (if (`self.chasing`)
    (cast `/Game/ThirdPerson/Blueprints/BP_RaccoonCharacter` _returnvalue)
    (`|AIMoveTo` self (`self.K2_GetActorLocation` _returnvalue) null)))

(fn `chase`)

(fn `UserConstructionScript`)
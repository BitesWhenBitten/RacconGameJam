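; Patrol point holder for enemy AI that supplies locations from its Locations array one at a time.
; GetNextLocation returns the entry at the current Index, then increments it for the next call.
; Index resets to zero only once it exceeds the array length, so it can land one past the last element before wrapping.
; BeginPlay and Tick are unused.
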(fn `GetNextLocation`
  (returns (NextLoxation :type "Vector Structure"))
  (bind _locations (`self.Locations`))
  (bind _index (`self.Index`))
  (bind _output_get (set `self.Output` (`|GetArrayItem` _locations _index)))
  (bind _result (`/Engine/EditorBlueprintResources/StandardMacros.IncrementInt` _index)
    (:`  `
      (if (> _result (`KismetArrayLibrary.Array_Length` _locations))
        (set `self.Index` 0)
        (else
          (set `self.Index` _result)))
      (return _output_get))))